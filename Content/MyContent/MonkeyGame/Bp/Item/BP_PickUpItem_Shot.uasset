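; Shot pickup item in MonkeyGame that switches the shot mode of the character that picks it up.
; It overrides the parent's PickUpItem event, runs the parent logic, then casts the actor to BP_ThirdPersonCharacter_copy and calls ChangeShotMode with a fixed enum value.
; Other actors get only the parent behavior, and the construction script just calls the parent.
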(event EventBeginPlay
  (|CallParentFunction) ; This node is disabled and will not be called.\nDrag off pins to build functionality.
)

(event Collision|EventActorBeginOverlap
  (params (OtherActor :type Actor%20Object%20Reference))
  (|CallParentFunction OtherActor) ; This node is disabled and will not be called.\nDrag off pins to build functionality.
)

(event EventTick
  (params (DeltaSeconds :type Float%20%28single-precision%29))
  (|CallParentFunction DeltaSeconds) ; This node is disabled and will not be called.\nDrag off pins to build functionality.
)

(event EventPickUpItem
  (params (Actor :type Actor%20Object%20Reference))
  (|CallParentFunction Actor)
  (bind _asbp_third_person_character_copy (Utilities|Casting|CastToBP_ThirdPersonCharacter_copy Actor))
  (Default|ChangeShotMode _asbp_third_person_character_copy "NewEnumerator2"))

(fn ConstructionScript
  (|CallParentFunction))