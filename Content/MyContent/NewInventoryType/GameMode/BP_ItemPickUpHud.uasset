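; HUD-style Blueprint for item pickup that creates the inventory widget, toggles it with cursor and input mode, and handles picking up and dropping items.
; Pickups join a non-full stack of the same class via interface messages, or become new item widgets in the wrap box.
; Each addition calls the game instance's SavedInventory with a separately created ItemBox widget.
; Drops spawn the item class ahead of the player and send it a message.
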(event Custom|Inventory_Off
  ;[1 1 1] InventoryWidget_Off
  (Widget|RemovefromParent (Variables|Widget|GetInventoryWidget))
  (Input|SetInputModeGameOnly (Game|GetPlayerController 0) false)
  (Variables|/Script/Engine.PlayerController|SetbShowMouseCursor (Game|GetPlayerController 0) false))

(event Custom|InventoryOn
  ;[1 1 1] InventoryWidget_On
  (UserInterface|Viewport|AddtoViewport (Variables|Widget|GetInventoryWidget) 0)
  (Input|SetInputModeGameandUI (Game|GetPlayerController 0) (Variables|Widget|GetInventoryWidget) "DoNotLock" true false)
  (Variables|/Script/Engine.PlayerController|SetbShowMouseCursor (Game|GetPlayerController 0) true))

(event EventBeginPlay
  ;[1 1 1] Init
  (bind _returnvalue (UserInterface|CreateWidget "/Game/MyContent/NewInventoryType/WBP/WBP_BaseWidget_InventorySystem.WBP_BaseWidget_InventorySystem_C"))
  (Variables|Widget|SetInventoryWidget _returnvalue)
  (bind _returnvalue_2 (UserInterface|CreateWidget "/Game/MyContent/NewInventoryType/WBP/WBP_ItemBox.WBP_ItemBox_C"))
  (Variables|Default|SetItemBox _returnvalue_2))

(event EventPickupItem
  (params (ItemClass :type Actor%20Class%20Reference) (ItemIcon :type Texture%202D%20Object%20Reference) (StackAmount :type Integer))
  ;[1 1 1] ItemLogic
  (CallFunction|AddItemTonInventory ItemClass ItemIcon StackAmount))

(event EventDropItem
  (params (ItemClass :type Actor%20Class%20Reference))
  (bind _returnvalue (Game|Player|GetPlayerPawn 0))
  ;[1 1 1] ItemLogic
  (bind _returnvalue_2 (Game|SpawnActorfromClass ItemClass (Math|Transform|MakeTransform (+ (Transformation|GetActorLocation _returnvalue) (* (Math|Vector|GetForwardVector (Transformation|GetActorRotation _returnvalue)) 3e+02)) "0, 0, 0" "2.000000,2.000000,2.000000") "AdjustIfPossibleButAlwaysSpawn" "MultiplyWithRoot" 0 0))
  (Class|BIItemInteract|PushPickUpItem(Message) _returnvalue_2))

(fn ConstructionScript)

(fn AddItemTonInventory
  (params (Local_ItemData :type Actor%20Class%20Reference) (Local_Item%20Icon :type Texture%202D%20Object%20Reference) (Local_Stack%20Amount :type Integer))
  (Variables|Local|SetLocal_Item%20Icon Local_Item%20Icon)
  (Variables|Local|SetLocal_ItemData Local_ItemData)
  (Variables|Local|SetLocal_Stack%20Amount Local_Stack%20Amount)
  (if (> (Variables|Local|GetLocal_Stack%20Amount) 1)
    (bind _array_element (Utilities|Array|ForEachLoopwithBreak (Class|PanelWidget|GetAllChildren (Variables|/Game/MyContent/NewInventoryType/WBP/WBP_ItemBox.WBP_ItemBox_C|GetInventoryBox (Variables|/Game/MyContent/NewInventoryType/WBP/WBP_BaseWidget_InventorySystem.WBP_BaseWidget_InventorySystem_C|GetWBP_ItemBox (Variables|Widget|GetInventoryWidget)))) :!label _label)
      (:LoopBody
        (bind _output_get (Variables|Local|SetLocal_Array%20Element _array_element))
        (bind (_itemclass _currentstaakamount _maxstackamount) (Class|BIItemInteract|GetPickUpItemData(Message) _output_get))
        (if (== _itemclass (Variables|Local|GetLocal_ItemData))
          (if (<= (+ _currentstaakamount 1) _maxstackamount)
            (Class|BIItemInteract|AddPickUpItemtoStack(Message) (Variables|Local|GetLocal_Array%20Element))
            (Variables|Default|SetbIsItemAdd true)
            (Default|SavedInventory (.AsBP%20Game%20Instance%20Item%20Pick%20Up (Utilities|Casting|CastToBP_GameInstance_ItemPickUp (Game|GetGameInstance))) (Variables|Default|GetItemBox) (Variables|Local|GetLocal_ItemData))
            (goto _label Break))))
      (:Completed
        (if (not (Variables|Default|GetbIsItemAdd))
          (bind _returnvalue (UserInterface|CreateWidget "/Game/MyContent/NewInventoryType/WBP/WBP_PickUpItem.WBP_PickUpItem_C" :!label _label_2))
          (bind _output_get_2 (Variables|Widget|SetWBP_PickUpItem _returnvalue))
          (Variables|/Game/MyContent/NewInventoryType/WBP/WBP_PickUpItem.WBP_PickUpItem_C|SetActorClass _output_get_2 (Variables|Local|GetLocal_ItemData))
          (Class|Image|SetBrush (Variables|/Game/MyContent/NewInventoryType/WBP/WBP_PickUpItem.WBP_PickUpItem_C|GetItemIcon _returnvalue) (Class|WidgetBlueprintLibrary|MakeBrushfromTexture (Variables|Local|GetLocal_Item%20Icon) 100 100))
          (Variables|/Game/MyContent/NewInventoryType/WBP/WBP_PickUpItem.WBP_PickUpItem_C|SetMaxStack (Variables|Widget|GetWBP_PickUpItem) (Variables|Local|GetLocal_Stack%20Amount))
          (Class|WrapBox|AddChildtoWrapBox (Variables|/Game/MyContent/NewInventoryType/WBP/WBP_ItemBox.WBP_ItemBox_C|GetInventoryBox (Variables|/Game/MyContent/NewInventoryType/WBP/WBP_BaseWidget_InventorySystem.WBP_BaseWidget_InventorySystem_C|GetWBP_ItemBox (Variables|Widget|GetInventoryWidget))) (Variables|Widget|GetWBP_PickUpItem))
          (Default|SavedInventory (.AsBP%20Game%20Instance%20Item%20Pick%20Up (Utilities|Casting|CastToBP_GameInstance_ItemPickUp (Game|GetGameInstance))) (Variables|Default|GetItemBox) (Variables|Local|GetLocal_ItemData)))))
    (else
      (goto _label_2))))

(fn GetPickUpItemData
  (return 0 0 0))

(fn Inventory
  (return (Variables|Default|GetItemBox)))