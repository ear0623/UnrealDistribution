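; Game instance that saves picked-up item data for an inventory system.
; Init creates a BP_Savegame_InventorySystem object and loads its slot into a separate reference, falling back to the new object.
; PickupItem writes class, icon and stack amount into the newly created object, not the loaded one, overwriting a single item record on disk.
; SavedInventory, Inventory and GetPickUpItemData are empty stubs.
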(event EventSavedInventory
  (params (LoadWidget :type Widget%20Object%20Reference) (ClassItem :type Actor%20Class%20Reference)))

(event EventInit
  (bind _returnvalue (SaveGame|CreateSaveGameObject "/Game/MyContent/NewInventoryType/SaveGame/BP_Savegame_InventorySystem.BP_Savegame_InventorySystem_C"))
  (Variables|Default|SetInventoryGame _returnvalue)
  (bind _returnvalue_2 (SaveGame|LoadGamefromSlot (Variables|/Game/MyContent/NewInventoryType/SaveGame/BP_Savegame_InventorySystem.BP_Savegame_InventorySystem_C|GetSlotName (Variables|Default|GetInventoryGame)) (Variables|/Game/MyContent/NewInventoryType/SaveGame/BP_Savegame_InventorySystem.BP_Savegame_InventorySystem_C|GetUserIndex (Variables|Default|GetInventoryGame))))
  (bind _asbp_savegame_inventory_system (Utilities|Casting|CastToBP_Savegame_InventorySystem _returnvalue_2)
    (:then
      (Variables|Default|SetAs%20BP%20Savegame%20Inventory%20System _asbp_savegame_inventory_system))
    (:CastFailed
      (Variables|Default|SetAs%20BP%20Savegame%20Inventory%20System (Variables|Default|GetInventoryGame)))))

(event EventPickupItem
  (params (ItemClass :type Actor%20Class%20Reference) (ItemIcon :type Texture%202D%20Object%20Reference) (StackAmount :type Integer))
  (bind _inventorygame (Variables|Default|GetInventoryGame))
  (Variables|/Game/MyContent/NewInventoryType/SaveGame/BP_Savegame_InventorySystem.BP_Savegame_InventorySystem_C|SetItemTextrue2D (Variables|Default|GetInventoryGame) ItemIcon)
  (Variables|/Game/MyContent/NewInventoryType/SaveGame/BP_Savegame_InventorySystem.BP_Savegame_InventorySystem_C|SetStackSize (Variables|Default|GetInventoryGame) StackAmount)
  (Variables|/Game/MyContent/NewInventoryType/SaveGame/BP_Savegame_InventorySystem.BP_Savegame_InventorySystem_C|SetItemClass _inventorygame ItemClass)
  (bind _returnvalue (SaveGame|SaveGametoSlot _inventorygame (Variables|/Game/MyContent/NewInventoryType/SaveGame/BP_Savegame_InventorySystem.BP_Savegame_InventorySystem_C|GetSlotName _inventorygame) (Variables|/Game/MyContent/NewInventoryType/SaveGame/BP_Savegame_InventorySystem.BP_Savegame_InventorySystem_C|GetUserIndex _inventorygame)))
  (Development|PrintString (Utilities|String|ToString(Boolean) _returnvalue)))

(fn GetPickUpItemData
  (return 0 0 0))

(fn Inventory
  (return 0))