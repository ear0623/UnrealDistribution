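; Default pawn for the inventory system that handles input for toggling the inventory and changing level.
; On BeginPlay it caches BP_ItemPickUpHud, and the WidgetToggle action alternates its InventoryOn and InventoryOff calls through a FlipFlop.
; The 1 key asks BP_ItemPickUpGameMode to open a level by name, but only when that game mode's Success flag is set.
; GetPickUpItemData is a stub returning zero stack amounts.
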(event EventBeginPlay
  ;[1 1 1] Init
  (bind _asbp_item_pick_up_hud (Utilities|Casting|CastToBP_ItemPickUpHud (HUD|GetHUD (Game|GetPlayerController 0))))
  (Variables|Hud|SetAs%20BP%20Item%20Pick%20Up%20Hud _asbp_item_pick_up_hud))

(event Collision|EventActorBeginOverlap
  (params (OtherActor :type Actor%20Object%20Reference)))

(event EventTick
  (params (DeltaSeconds :type Float%20%28single-precision%29)))

(event Input|ActionEvents|InputActionWidgetToggle
  (params (Key :type Key%20Structure :default "None"))
  (bind _as_bp_item_pick_up_hud (Variables|Hud|GetAs%20BP%20Item%20Pick%20Up%20Hud))
  ;[1 1 1] InventoryOnOff
  (:Pressed
    (Utilities|FlowControl|FlipFlop
      (:A
        (Default|Inventoryon _as_bp_item_pick_up_hud))
      (:B
        (Default|InventoryOff _as_bp_item_pick_up_hud)))))

(event Input|KeyboardEvents|1
  (params (Key :type Key%20Structure :default "None"))
  (bind _returnvalue (Game|GetGameMode))
  (bind (_asbp_item_pick_up_game_mode _bsuccess) (Utilities|Casting|CastToBP_ItemPickUpGameMode _returnvalue))
  (:Pressed
    (if _bsuccess
      (Default|OpenLevel _asbp_item_pick_up_game_mode))))

(fn ConstructionScript)

(fn GetPickUpItemData
  (return 0 0 0))