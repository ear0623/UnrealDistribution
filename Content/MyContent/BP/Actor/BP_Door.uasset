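; BP_Door is an interactive door actor that the player opens and closes with the E key.
; Box overlap with a DefaultPawn enables the actor's input and shows a PointLight; leaving disables input and hides it.
; E calls ActionDoor, where a FlipFlop alternately plays and reverses the DoorOnOff timeline, whose OnOff track drives the StaticMesh's relative yaw.
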(event OnComponentBeginOverlap(Box)
  (params (OverlappedComponent :type Primitive%20Component%20Object%20Reference) (OtherActor :type Actor%20Object%20Reference) (OtherComp :type Primitive%20Component%20Object%20Reference) (OtherBodyIndex :type Integer) (bFromSweep :type Boolean) (SweepResult :type Hit%20Result%20Structure%20%28by%20ref%29))
  ;[1 1 1] OverrapIvent
  (Utilities|Casting|CastToDefaultPawn OtherActor)
  (Input|EnableInput (Game|GetPlayerController 0))
  (Rendering|SetVisibility (Variables|Default|GetPointLight) true false))

(event OnComponentEndOverlap(Box)
  (params (OverlappedComponent :type Primitive%20Component%20Object%20Reference) (OtherActor :type Actor%20Object%20Reference) (OtherComp :type Primitive%20Component%20Object%20Reference) (OtherBodyIndex :type Integer))
  ;[1 1 1] OverrapIvent
  (Utilities|Casting|CastToDefaultPawn OtherActor)
  (Input|DisableInput (Game|GetPlayerController 0))
  (Rendering|SetVisibility (Variables|Default|GetPointLight) false false))

(event Custom|ActionDoor
  ;[1 1 1] Animation
  (Utilities|FlowControl|FlipFlop
    (:A
      (bind _onoff (Timeline|DoorOnOff Play)
        (:Update
          (Transformation|SetRelativeRotation (Variables|Default|GetStaticMesh) (Math|Rotator|MakeRotator 0.0 0.0 _onoff) false false))))
    (:B
      (Timeline|DoorOnOff Reverse))))

(event EventBeginPlay)

(event Collision|EventActorBeginOverlap
  (params (OtherActor :type Actor%20Object%20Reference)))

(event EventTick
  (params (DeltaSeconds :type Float%20%28single-precision%29)))

(event Input|KeyboardEvents|E
  (params (Key :type Key%20Structure :default "None"))
  ;[1 1 1] OverrapIvent
  (:Pressed
    (CallFunction|ActionDoor)))

(fn ConstructionScript)