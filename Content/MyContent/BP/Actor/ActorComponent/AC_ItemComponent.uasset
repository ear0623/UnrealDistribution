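; AC_ItemComponent is an actor component that moves items into an inventory.
; SaveItemtoInventory stores the given item in ItemData.
; ItemtoInventory appends the class of a valid ItemData to the inventory class list and passes that list to the base widget to update the inventory.
; SpawnItem is declared as an empty stub.
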(event Custom|Item%20to%20Inventory
  ;[1 1 1] Item to inventory
  (Utilities|IsValid (Variables|Item|GetItemData)
    (:Is%20Valid
      (Utilities|Array|Add (Variables|Local|GetBaseItemClass_InInventory) (Utilities|GetClass (Variables|Item|GetItemData)))
      (Default|FAddFuntionInventory (Variables|Widgwt|GetBaseWidget) (Variables|Local|GetBaseItemClass_InInventory)))))

(event Custom|SaveItemtoInventory
  (params (ItemData :type Base%20Item%20Object%20Reference))
  ;[1 1 1] ItemToInventory
  (Variables|Item|SetItemData ItemData))

(event Custom|SpawnItem
  ;[1 1 1] OutputItem
)