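; Game instance that holds the player's best time and a count, backed by an SG_Time save object.
; Init loads both values from the save slot, falling back to a fresh save object when none exists.
; SetBestTime stores and saves values at least as high as the current best, while SetCount only updates memory.
; Inventory saving is unfinished: SavedInventory and Inventory are empty, and the inventory save logic is disconnected.
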(event Custom|Set%20BestTime
  (params (A :type Float%20%28double-precision%29))
  (bind _as_sg_time (Variables|Default|GetAs%20SG%20Time))
  ;[1 1 1] Save
  (if (>= A (Variables|Default|GetBestTime))
    (bind _output_get (Variables|Default|SetBestTime A))
    (Variables|/Game/MyContent/SaveGames/SG_Time.SG_Time_C|SetBestTime (Variables|Default|GetAs%20SG%20Time) _output_get)
    (bind _returnvalue (SaveGame|SaveGametoSlot (Variables|Default|GetAs%20SG%20Time) (Variables|/Game/MyContent/SaveGames/SG_Time.SG_Time_C|GetSlotName _as_sg_time) (Variables|/Game/MyContent/SaveGames/SG_Time.SG_Time_C|GetUserIndex _as_sg_time)))
    (Development|PrintString (Utilities|String|Append "Saved" (Utilities|String|ToString(Boolean) _returnvalue)))))

(event EventSavedInventory
  (params (LoadWidget :type Widget%20Object%20Reference) (ClassItem :type Actor%20Class%20Reference)))

(event EventSetCount
  (params (Value :type Integer))
  (bind _output_get (Variables|Default|SetCount Value))
  (Development|PrintString (Utilities|String|ToString(Integer) _output_get)))

(event EventInit
  ;[1 1 1] Load
  (bind _returnvalue (SaveGame|CreateSaveGameObject "/Game/MyContent/SaveGames/SG_Time.SG_Time_C"))
  (bind _returnvalue_2 (SaveGame|LoadGamefromSlot (Variables|/Game/MyContent/SaveGames/SG_Time.SG_Time_C|GetSlotName _returnvalue) (Variables|/Game/MyContent/SaveGames/SG_Time.SG_Time_C|GetUserIndex _returnvalue)))
  (bind _assg_time (Utilities|Casting|CastToSG_Time _returnvalue_2)
    (:then
      (bind _output_get (Variables|Default|SetAs%20SG%20Time _assg_time))
      (Variables|Default|SetBestTime (Variables|/Game/MyContent/SaveGames/SG_Time.SG_Time_C|GetBestTime _output_get))
      (Variables|Default|SetCount (Variables|/Game/MyContent/SaveGames/SG_Time.SG_Time_C|GetCount _output_get)))
    (:CastFailed
      (Variables|Default|SetAs%20SG%20Time _returnvalue))))

(fn GetCount
  (return (Variables|Default|GetCount)))

(fn Inventory
  (return 0))